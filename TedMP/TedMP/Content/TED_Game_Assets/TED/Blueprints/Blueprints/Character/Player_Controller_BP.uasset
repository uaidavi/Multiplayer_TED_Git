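; Player controller for Personagem_Generico_BP that handles movement, double jump, spring-arm camera orbit and respawning.
; Pan input rotates the pitch-clamped spring arm, and when movement starts a timeline lerps control rotation toward it.
; Sideways input strafes while moving but turns in place when still.
; Pawn destruction triggers a delayed respawn through Modo01, then re-possesses and re-caches references; a test key zeroes health.
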(event `self.ReceiveTick`
  (params (DeltaSeconds :type "Float (single-precision)"))
  (`self.Char_Rot_Call`))

(event `RespawnReset`
  (`KismetSystemLibrary.Delay` 0.1 :!label _label)
  (`self.GetReferences`)
  (`self.Teste`))

(event `self.ReceiveBeginPlay`
  (goto _label))

(event `InputAxis|PanHor`
  (params (AxisValue :type "Float (single-precision)"))
  (`self.Validation_Macro`
    (:`Is Valid`
      (`self.CamRotationX` (`self.Cast_Char`) AxisValue))))

(event `InputAxis|PanVert`
  (params (AxisValue :type "Float (single-precision)"))
  (`self.Validation_Macro`
    (:`Is Valid`
      (`self.CamRotationY` (`self.Cast_Char`) AxisValue))))

(event `InputAxis|RunForward`
  (params (AxisValue :type "Float (single-precision)"))
  (`self.Validation_Macro`
    (:`Is Valid`
      (`self.MoveForward` (`self.Cast_Char`) AxisValue))))

(event `Char_Rot_Call`
  ;[1 1 1] Char_Rot_Behavior
  (`self.Validation_Macro`
    (:`Is Valid`
      (if (`self.VelocityTest`)
        (if (and (`self.VelocityTest`) (`self.StartedMov`))
          (bind _char_initial_rot (`self.Create_Char_InitialRot`)
            (:`Exec`
              (set `self.Char_Init_Rot` _char_initial_rot)
              (bind (_direction _rot_alpha) (`Timeline|Timeline_0` :!via `PlayFromStart`)
                (:`Update`
                  (`self.SetControlRotation` (`KismetMathLibrary.RLerp` (`self.Char_Init_Rot`) (`SceneComponent.RelativeRotation` (`self.CamHold`)) _rot_alpha true))
                  (set `self.StartedMov` false))))))
        (else
          ;;[1 1 1] RestartStartedMoving
          (set `self.StartedMov` true))))))

(event `InputAxis|MoveTurnSide`
  (params (AxisValue :type "Float (single-precision)"))
  (`self.Validation_Macro`
    (:`Is Valid`
      (`self.MoveSideways` (`self.Cast_Char`) AxisValue))))

(event `InputAction|Jump_Inp`
  (params (Key :type "Key Structure" :default "AnyKey"))
  (:`Pressed`
    (`self.Validation_Macro`
      (:`Is Valid`
        (bind _aspersonagem_generico_bp (cast `/Game/TED_Game_Assets/TED/Blueprints/Blueprints/Character/Personagem_Generico_BP` (`self.K2_GetPawn`)))
        (`/Game/TED_Game_Assets/TED/Blueprints/Blueprints/Character/Personagem_Generico_BP.DoubleJump` _aspersonagem_generico_bp)))))

(event `Teste`
  (bind _returnvalue (`self.K2_GetPawn`))
  (`/Engine/EditorBlueprintResources/StandardMacros.IsValid` _returnvalue
    (:`Is Valid`
      (add `self.OnDestroyed` _returnvalue (delegate `RequestServerSpawn`)))))

(event `RequestServerSpawn`
  (`KismetSystemLibrary.Delay` 2.0)
  (`self.RespawnSequence`)
  (`self.RespawnReset`))

(event `InputAction|BotaoTeste`
  (params (Key :type "Key Structure" :default "AnyKey"))
  (:`Pressed`
    (bind _aspersonagem_generico_bp (cast `/Game/TED_Game_Assets/TED/Blueprints/Blueprints/Character/Personagem_Generico_BP` (`self.K2_GetPawn`)))
    (`KismetSystemLibrary.PrintString` "vou morrer")
    (set `/Game/TED_Game_Assets/TED/Blueprints/Blueprints/Character/Personagem_Generico_BP.CurHealth` 0.0 _aspersonagem_generico_bp)))

(fn `CamRotationX`
  (params (To_Char :type "/Game/TED_Game_Assets/TED/Blueprints/Blueprints/Character/Personagem_Generico_BP Object Reference") (Axis :type "Float (double-precision)"))
  (`SceneComponent.K2_AddRelativeRotation` (`self.CamHold`) (`KismetMathLibrary.MakeRotator` 0.0 0.0 Axis) false false)
  (if (`self.VelocityTest`)
    (`Pawn.AddControllerYawInput` To_Char (* Axis 0.4)))
  (return))

(fn `CamRotationY`
  (params (To_Char :type "/Game/TED_Game_Assets/TED/Blueprints/Blueprints/Character/Personagem_Generico_BP Object Reference") (Axis_Value :type "Float (double-precision)"))
  (bind (_newparam _toohigh _toolow) (`self.Camera_Rot_Test`))
  (bind _camhold (`self.CamHold`))
  (bind _camhold_2 (`self.CamHold`))
  (bind (_relativerotation_roll _relativerotation_pitch _relativerotation_yaw) (`KismetMathLibrary.BreakRotator` (`SceneComponent.RelativeRotation` _camhold)))
  (bind (_relativerotation_roll_2 _relativerotation_pitch_2 _relativerotation_yaw_2) (`KismetMathLibrary.BreakRotator` (`SceneComponent.RelativeRotation` _camhold_2)))
  (`self.Validation_Macro`
    (:`Is Valid`
      (if _toohigh
        ;[1 1 1] High_Rot_Correction
        (`SceneComponent.K2_SetRelativeRotation` _camhold_2 (`KismetMathLibrary.MakeRotator` _relativerotation_roll_2 -47.99 _relativerotation_yaw_2) false false)
        (elif _toolow
          ;[1 1 1] Low_Rot_Correction
          (`SceneComponent.K2_SetRelativeRotation` _camhold (`KismetMathLibrary.MakeRotator` _relativerotation_roll 47.99 _relativerotation_yaw) false false)
          (else
            (`SceneComponent.K2_AddRelativeRotation` (`self.CamHold`) (`KismetMathLibrary.MakeRotator` 0.0 Axis_Value) false false)))))
    (:`Char Is Not Valid`
      _)
    (:`Cam Is Not Valid`
      _))
  (return))

(fn `ControllerDeathBehavior`
  (`self.UnPossess`)
  (bind _asmodo_01 (cast `/Game/TED_Game_Assets/GameInfo/Modo01` (`GameplayStatics.GetGameMode`)))
  (`/Game/TED_Game_Assets/GameInfo/Modo01.Request_Respawn` _asmodo_01 self))

(fn `GetReferences`
  (bind _returnvalue (`self.K2_GetPawn`))
  (`/Engine/EditorBlueprintResources/StandardMacros.IsValid` _returnvalue
    (:`Is Valid`
      (bind _aspersonagem_generico_bp (cast `/Game/TED_Game_Assets/TED/Blueprints/Blueprints/Character/Personagem_Generico_BP` _returnvalue)
        (:`then`
          (`Character.Jump` _aspersonagem_generico_bp)
          (`/Engine/EditorBlueprintResources/StandardMacros.IsValid` _aspersonagem_generico_bp
            (:`Is Valid`
              (bind _output_get (set `self.Cast_Char` _aspersonagem_generico_bp))
              (`/Engine/EditorBlueprintResources/StandardMacros.IsValid` _output_get
                (:`Is Valid`
                  (set `self.CamHold` (`/Game/TED_Game_Assets/TED/Blueprints/Blueprints/Character/Personagem_Generico_BP.SpringArm` _aspersonagem_generico_bp)))
                (:`Is Not Valid`
                  (`KismetSystemLibrary.PrintString` "Set Char Invalido" true true (struct :`G` 1.0 :`B` 0.095112 :`A` 1.0) 30.0)
                  (`KismetSystemLibrary.PrintString` "AlgoEstáInvalido" true true (struct :`R` 1.0 :`G` 0.81113 :`A` 1.0) 90.0 :!label _label))))
            (:`Is Not Valid`
              (`KismetSystemLibrary.PrintString` "personagem invalido" true true (struct :`G` 1.0 :`B` 0.095112 :`A` 1.0) 30.0)
              (goto _label))))
        (:`CastFailed`
          (`KismetSystemLibrary.PrintString` "Cast Fail" true true (struct :`R` 1.0 :`B` 0.05564 :`A` 1.0) 90.0)
          (goto _label))))
    (:`Is Not Valid`
      (`KismetSystemLibrary.PrintString` "NAO TENHO UM PAWN" true true (struct :`R` 0.77 :`A` 1.0) 20.0)
      (goto _label)))
  (return))

(fn `MoveForward`
  (params (To_Char :type "/Game/TED_Game_Assets/TED/Blueprints/Blueprints/Character/Personagem_Generico_BP Object Reference") (`FWD/BWD` :type "Float (double-precision)"))
  (`self.Validation_Macro`
    (:`Is Valid`
      (if (not (`self.IsIncapacitated`))
        (`Pawn.AddMovementInput` To_Char (`KismetMathLibrary.GetForwardVector` (`KismetMathLibrary.MakeRotator` 0.0 0.0 (.yaw (`self.GetControlRotation`)))) (* `FWD/BWD` 1.0) false)))
    (:`Char Is Not Valid`
      _)
    (:`Cam Is Not Valid`
      _))
  (return))

(fn `MoveSideways`
  (params (To_Char :type "/Game/TED_Game_Assets/TED/Blueprints/Blueprints/Character/Personagem_Generico_BP Object Reference") (Axis_Value :type "Float (double-precision)"))
  (if (`self.VelocityTest`)
    (`Pawn.AddMovementInput` To_Char (`KismetMathLibrary.GetRightVector` (`KismetMathLibrary.MakeRotator` 0.0 0.0 (.yaw (`self.GetControlRotation`)))) Axis_Value false)
    (else
      (`Pawn.AddControllerYawInput` To_Char Axis_Value)))
  (return))

(fn `RespawnSequence`
  (bind _asmodo_01 (cast `/Game/TED_Game_Assets/GameInfo/Modo01` (`GameplayStatics.GetGameMode`))
    (:`then`
      (bind _newchar (`/Game/TED_Game_Assets/GameInfo/Modo01.Request_Respawn` _asmodo_01 self))
      (`self.Possess` _newchar))
    (:`CastFailed`
      _))
  (return))

(fn `UserConstructionScript`)