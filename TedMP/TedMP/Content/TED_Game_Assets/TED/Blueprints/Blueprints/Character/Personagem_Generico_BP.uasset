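; Generic character Blueprint that handles death and declares mostly empty hooks for attacks, block, riposte and respawn.
; Tick polls CurHealth and, at exactly zero, fires DeathEvent, which runs DeathBehavior and destroys the actor.
; DeathBehavior rechecks health on the authority and unpossesses the Player_Controller_BP before destruction.
; DoubleJump simply calls Jump, StringTest prints debug strings, and the health de-buff OnRep is empty.
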(event `self.ReceiveBeginPlay`)

(event `self.ReceiveActorBeginOverlap`
  (params (OtherActor :type "Actor Object Reference")))

(event `self.ReceiveTick`
  (params (DeltaSeconds :type "Float (single-precision)"))
  (if (== (`self.CurHealth`) 0.0)
    (`KismetSystemLibrary.PrintString` "Morri")
    (`self.DeathEvent`)))

(event `DeathEvent`
  (`self.Death_Behavior`)
  (`self.K2_DestroyActor`))

(fn `Atk1_Call`)

(fn `Atk2_Call`)

(fn `BlockCall`)

(fn `Death_Behavior`
  (`/Engine/EditorBlueprintResources/ActorMacros.Switch Has Authority`
    (:`Authority`
      (if (== (`self.CurHealth`) 0.0)
        (`KismetSystemLibrary.PrintString` "Morri")
        (bind _asplayer_controller_bp (cast `/Game/TED_Game_Assets/TED/Blueprints/Blueprints/Character/Player_Controller_BP` (`self.GetController`))
          (:`then`
            (`Controller.UnPossess` _asplayer_controller_bp))
          (:`CastFailed`
            _))))
    (:`Remote`
      _))
  (return))

(fn `DoubleJump`
  (`self.Jump`))

(fn `OnRep_Health_De-Buff`)

(fn `Respawn_Behavior`)

(fn `RiposteCall`)

(fn `StringTest`
  (for _array_element _
    (`KismetSystemLibrary.PrintString` _array_element true true (struct :`G` 0.66 :`B` 1.0 :`A` 1.0) 5.0)))

(fn `UserConstructionScript`)