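; Generic playable character (apparently a backup) with control-yaw-relative movement, jump and an orbiting spring-arm camera.
; Camera input rotates the arm with clamped pitch and also yaws the controller while moving; side input strafes when moving, turns when stationary.
; Tick zeroes camera roll and, as movement starts, runs a timeline lerping control rotation toward the arm's rotation.
; Zero health only prints a debug message; attack, block, riposte and respawn are empty stubs.
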(event `InputAxis|PanHor`
  (params (AxisValue :type "Float (single-precision)"))
  (`self.Cam_Rotation_X` AxisValue))

(event `Char_Rot_Call`
  ;[1 1 1] Char_Rot_Behavior
  (if (`self.VelocityTest`)
    (if (and (`self.VelocityTest`) (`self.StartedMov`))
      (set `self.Char_Init_Rot` (struct))
      (bind (_direction _rot_alpha) (`Timeline|Char_Rot_Value` :!via `PlayFromStart`)
        (:`Update`
          (`Controller.SetControlRotation` (`GameplayStatics.GetPlayerController` 0) (`KismetMathLibrary.RLerp` (`self.Char_Init_Rot`) (`SceneComponent.RelativeRotation` (`self.SpringArm`)) _rot_alpha true))
          (set `self.StartedMov` false))))
    (else
      ;;[1 1 1] RestartStartedMoving
      (set `self.StartedMov` true))))

(event `/Game/TED_Game_Assets/TED/Blueprints/Blueprints/Character/Personagem_Generico_BP.ReceiveBeginPlay`)

(event `InputAxis|PanVert`
  (params (AxisValue :type "Float (single-precision)"))
  (`self.Cam_Rotation_Y` AxisValue))

(event `self.ReceiveActorBeginOverlap`
  (params (OtherActor :type "Actor Object Reference")))

(event `InputAxis|RunForward`
  (params (AxisValue :type "Float (single-precision)"))
  (`self.MoveForward` AxisValue))

(event `/Game/TED_Game_Assets/TED/Blueprints/Blueprints/Character/Personagem_Generico_BP.ReceiveTick`
  (params (DeltaSeconds :type "Float (single-precision)"))
  (if (== (`self.CurHealth`) 0.0)
    (`self.DeathEvent`)
    (else
      (`self.Correct_Cam_Roll`)
      (`self.Char_Rot_Call`))))

(event `InputAxis|MoveTurnSide`
  (params (AxisValue :type "Float (single-precision)"))
  (`self.MoveSideways` AxisValue))

(event `DeathEvent`
  (`self.Death_Behavior`))

(event `InputAction|Jump_Inp`
  (params (Key :type "Key Structure" :default "AnyKey"))
  (:`Pressed`
    (`self.DoubleJump` null)))

(fn `Atk1_Call`)

(fn `Atk2_Call`)

(fn `BlockCall`)

(fn `Cam_Rotation_X`
  (params (X_Axis_Value :type "Float (double-precision)"))
  (`SceneComponent.K2_AddRelativeRotation` (`self.SpringArm`) (`KismetMathLibrary.MakeRotator` 0.0 0.0 X_Axis_Value) false false)
  (if (`self.VelocityTest`)
    (`self.AddControllerYawInput` (* X_Axis_Value 0.4)))
  (return))

(fn `Cam_Rotation_Y`
  (params (Y_Axis_Value :type "Float (double-precision)"))
  (bind (_can_rotv _toohigh _toolow) (`self.Test_Camera_Rot`))
  (bind _springarm (`self.SpringArm`))
  (bind (_relativerotation_roll _relativerotation_pitch _relativerotation_yaw) (`KismetMathLibrary.BreakRotator` (`SceneComponent.RelativeRotation` (`self.SpringArm`))))
  (bind (_relativerotation_roll_2 _relativerotation_pitch_2 _relativerotation_yaw_2) (`KismetMathLibrary.BreakRotator` (`SceneComponent.RelativeRotation` _springarm)))
  (if _toohigh
    ;[1 1 1] High_Rot_Correction
    (`SceneComponent.K2_SetRelativeRotation` _springarm (`KismetMathLibrary.MakeRotator` _relativerotation_roll_2 -47.99 _relativerotation_yaw_2) false false)
    (elif _toolow
      ;[1 1 1] Low_Rot_Correction
      (`SceneComponent.K2_SetRelativeRotation` (`self.SpringArm`) (`KismetMathLibrary.MakeRotator` _relativerotation_roll 47.99 _relativerotation_yaw) false false)
      (else
        (`SceneComponent.K2_AddRelativeRotation` (`self.SpringArm`) (`KismetMathLibrary.MakeRotator` 0.0 Y_Axis_Value) false false))))
  (return))

(fn `Correct_Cam_Roll`
  (bind _springarm (`self.SpringArm`))
  (bind (_relativerotation_roll _relativerotation_pitch _relativerotation_yaw) (`KismetMathLibrary.BreakRotator` (`SceneComponent.RelativeRotation` _springarm)))
  (`SceneComponent.K2_SetRelativeRotation` _springarm (`KismetMathLibrary.MakeRotator` 0.0 _relativerotation_pitch _relativerotation_yaw) false false))

(fn `Death_Behavior`
  (`/Engine/EditorBlueprintResources/ActorMacros.Switch Has Authority`
    (:`Authority`
      (if (== (`self.CurHealth`) 0.0)
        (`KismetSystemLibrary.PrintString` "Morri")))
    (:`Remote`
      _))
  (return))

(fn `DoubleJump`
  (params (To_Char :type "/Game/TED_Game_Assets/TED/Blueprints/Blueprints/Character/Personagem_Generico_BP Object Reference"))
  (`self.Jump` To_Char))

(fn `MoveForward`
  (params (`FWD/BWD` :type "Float (double-precision)"))
  (`self.AddMovementInput` (`KismetMathLibrary.GetForwardVector` (`KismetMathLibrary.MakeRotator` 0.0 0.0 (.yaw (`self.GetControlRotation`)))) (* `FWD/BWD` 1.0)))

(fn `MoveSideways`
  (params (Side :type "Float (double-precision)"))
  (if (`self.VelocityTest`)
    (`self.AddMovementInput` (`KismetMathLibrary.GetRightVector` (`KismetMathLibrary.MakeRotator` 0.0 0.0 (.yaw (`self.GetControlRotation`)))) Side)
    (else
      (`self.AddControllerYawInput` Side)))
  (return))

(fn `OnRep_Health_De-Buff`)

(fn `Respawn_Behavior`)

(fn `RiposteCall`)

(fn `StringTest`
  (for _array_element (`self.StringArray`)
    (`KismetSystemLibrary.PrintString` _array_element true true (struct :`G` 0.66 :`B` 1.0 :`A` 1.0) 5.0)))

(fn `UserConstructionScript`)